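; BP_Bull is an enemy bull hazard that starts charging as soon as play begins.
; ActivateBull loops the charge animation, adds audio and fades a warning material on the Pathing component.
; After a short delay, a timeline pushes the actor along world +X, lerping from its current location each update, so movement accumulates.
; Box overlap with BP_MainCharacter calls that character's BullHit.
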(event `self.ReceiveBeginPlay`
  (`self.Activate Bull`))

(event `self.Box.OnComponentBeginOverlap`
  (params (OverlappedComponent :type "PrimitiveComponent Object Reference") (OtherActor :type "Actor Object Reference") (OtherComp :type "PrimitiveComponent Object Reference") (OtherBodyIndex :type Integer) (bFromSweep :type Boolean) (SweepResult :type "HitResult Structure (by ref)"))
  (bind _asbp_main_character (cast `/Game/Characters/Car/BP_MainCharacter` OtherActor))
  (bind _output_get (set `self.Main Character Reference` _asbp_main_character))
  (`KismetSystemLibrary.PrintString` "Hit bull")
  (`/Game/Characters/Car/BP_MainCharacter.Bull Hit` _output_get))

(event `Activate Bull`
  (bind _returnvalue (`self.K2_GetActorLocation`))
  (`SkeletalMeshComponent.PlayAnimation` (`self.Bull`) "/Game/SM_Models/Bull/BullCharge_Anim.BullCharge_Anim" true)
  (`AddComponent|NODE_AddAudioComponent-0`)
  (`KismetSystemLibrary.PrintString` "Bull activated")
  (`|ExecutionSequence`
    (:`then_0`
      (`KismetSystemLibrary.Delay` 1.5)
      (bind (_direction _bull_running_at_player) (`Timeline|Timeline` :!via `PlayFromStart`)
        (:`Update`
          (`self.K2_SetActorLocation` (`KismetMathLibrary.VLerp` _returnvalue (+ _returnvalue (400.0 0.0 0.0)) _bull_running_at_player)))))
    (:`then_1`
      (bind _returnvalue_2 (`PrimitiveComponent.CreateDynamicMaterialInstance` (`self.Pathing`) 0 "/Game/Blueprints/Enemy/M_Warning.M_Warning" "None"))
      (bind (_direction_2 _fade_effect) (`Timeline|Fade Timeline`)
        (:`Update`
          (`MaterialInstanceDynamic.SetScalarParameterValue` _returnvalue_2 "Fade" _fade_effect))))))

(fn `UserConstructionScript`)