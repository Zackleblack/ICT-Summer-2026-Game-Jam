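; BP_Ukulele is a ukulele pickup that gives the player a buff through the HUD.
; A timeline started on BeginPlay spins its cone mesh in yaw at a slight fixed tilt.
; When BP_MainCharacter overlaps the Box, it prints a pickup message, then a DoOnce calls UkuleleBuff on the first WBP_HUD found and destroys the actor after a short delay.
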(event `self.ReceiveBeginPlay`
  (bind (_direction _rotate) (`Timeline|Timeline`)
    (:`Update`
      (`SceneComponent.K2_SetWorldRotation` (`self.Cone`) (`KismetMathLibrary.MakeRotator` 0.0 10.0 (`KismetMathLibrary.Lerp` 0.0 360.0 _rotate)) false false)
      (`SceneComponent.K2_SetWorldRotation` (`self.Cone`) (`KismetMathLibrary.MakeRotator` 0.0 10.0 (`KismetMathLibrary.Lerp` 0.0 360.0 _rotate)) false false))))

(event `self.Box.OnComponentBeginOverlap`
  (params (OverlappedComponent :type "PrimitiveComponent Object Reference") (OtherActor :type "Actor Object Reference") (OtherComp :type "PrimitiveComponent Object Reference") (OtherBodyIndex :type Integer) (bFromSweep :type Boolean) (SweepResult :type "HitResult Structure (by ref)"))
  (cast `/Game/Characters/Car/BP_MainCharacter` OtherActor)
  (`KismetSystemLibrary.PrintString` "Ukulele Picked Up")
  (`/Engine/EditorBlueprintResources/StandardMacros.DoOnce` false
    (:`Completed`
      (bind _foundwidgets (`WidgetBlueprintLibrary.GetAllWidgetsOfClass` "/Game/Widget/WBP_HUD.WBP_HUD_C"))
      (`/Game/Widget/WBP_HUD.UkuleleBuff` (`|GetArrayItem` _foundwidgets))
      (`KismetSystemLibrary.Delay` 0.2)
      (`self.K2_DestroyActor`))))

(fn `UserConstructionScript`)