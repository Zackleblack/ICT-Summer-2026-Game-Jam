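; BP_Pillow is a pickup that turns on the pillow mechanic for the main character who overlaps it.
; A timeline started at BeginPlay drives a full yaw spin of the tilted cone mesh.
; Box overlap waits briefly, casts to BP_MainCharacter and calls PillowOn, then destroys the pickup after another short delay.
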(event `self.ReceiveBeginPlay`
  (bind (_direction _rotate) (`Timeline|Timeline`)
    (:`Update`
      (`SceneComponent.K2_SetWorldRotation` (`self.Cone`) (`KismetMathLibrary.MakeRotator` -180.0 35.0 (`KismetMathLibrary.Lerp` 0.0 360.0 _rotate)) false false)
      (`SceneComponent.K2_SetWorldRotation` (`self.Cone`) (`KismetMathLibrary.MakeRotator` -180.0 35.0 (`KismetMathLibrary.Lerp` 0.0 360.0 _rotate)) false false))))

(event `self.Box.OnComponentBeginOverlap`
  (params (OverlappedComponent :type "PrimitiveComponent Object Reference") (OtherActor :type "Actor Object Reference") (OtherComp :type "PrimitiveComponent Object Reference") (OtherBodyIndex :type Integer) (bFromSweep :type Boolean) (SweepResult :type "HitResult Structure (by ref)"))
  ; Pillow Mechanic
  (`KismetSystemLibrary.Delay` 0.2)
  (bind _asbp_main_character (cast `/Game/Characters/Car/BP_MainCharacter` OtherActor))
  (`/Game/Characters/Car/BP_MainCharacter.Pillow On` _asbp_main_character)
  (`KismetSystemLibrary.Delay` 0.2)
  (`self.K2_DestroyActor`))

(fn `UserConstructionScript`)