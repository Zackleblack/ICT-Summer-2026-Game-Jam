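; BP_GasCan is a gas can pickup that the main character collects by overlapping its box.
; On BeginPlay a timeline drives the cone's yaw through a turn at a fixed pitch.
; Overlap by BP_MainCharacter prints a pickup message and calls RestartTimer, which, despite its name, only destroys the actor after a short delay.
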(event `self.ReceiveBeginPlay`
  (bind (_direction _rotate) (`Timeline|Timeline`)
    (:`Update`
      (`SceneComponent.K2_SetWorldRotation` (`self.Cone`) (`KismetMathLibrary.MakeRotator` 0.0 35.0 (`KismetMathLibrary.Lerp` 0.0 360.0 _rotate)) false false)
      (`SceneComponent.K2_SetWorldRotation` (`self.Cone`) (`KismetMathLibrary.MakeRotator` 0.0 35.0 (`KismetMathLibrary.Lerp` 0.0 360.0 _rotate)) false false))))

(event `self.Box.OnComponentBeginOverlap`
  (params (OverlappedComponent :type "PrimitiveComponent Object Reference") (OtherActor :type "Actor Object Reference") (OtherComp :type "PrimitiveComponent Object Reference") (OtherBodyIndex :type Integer) (bFromSweep :type Boolean) (SweepResult :type "HitResult Structure (by ref)"))
  (cast `/Game/Characters/Car/BP_MainCharacter` OtherActor)
  (`KismetSystemLibrary.PrintString` "Gascan Picked Up")
  (`self.Restart Timer`))

(event `Restart Timer`
  (`|ExecutionSequence`
    (:`then_0`
      (`KismetSystemLibrary.Delay` 0.2)
      (`self.K2_DestroyActor`))))

(fn `UserConstructionScript`)