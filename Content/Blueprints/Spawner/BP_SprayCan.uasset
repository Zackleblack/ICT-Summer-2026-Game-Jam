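; BP_SprayCan is a pickup that spawns a BP_Bull when the player collects it.
; A Timeline started on BeginPlay spins the tilted Cylinder around yaw.
; The first Box overlap passes a DoOnce, then a cast to BP_MainCharacter gates spawning the bull at StartPoint and destroying the can after a short delay.
; BeginPlay also caches an existing BP_Bull in BullReference, which this graph never reads.
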(event `self.ReceiveBeginPlay`
  (bind _returnvalue (`GameplayStatics.GetActorOfClass` "/Game/Blueprints/Enemy/BP_Bull.BP_Bull_C"))
  (set `self.Bull Reference` _returnvalue)
  (bind (_direction _rotate) (`Timeline|Timeline`)
    (:`Update`
      (`SceneComponent.K2_SetWorldRotation` (`self.Cylinder`) (`KismetMathLibrary.MakeRotator` -180.0 35.0 (`KismetMathLibrary.Lerp` 0.0 360.0 _rotate)) false false))))

(event `self.Box.OnComponentBeginOverlap`
  (params (OverlappedComponent :type "PrimitiveComponent Object Reference") (OtherActor :type "Actor Object Reference") (OtherComp :type "PrimitiveComponent Object Reference") (OtherBodyIndex :type Integer) (bFromSweep :type Boolean) (SweepResult :type "HitResult Structure (by ref)"))
  (`/Engine/EditorBlueprintResources/StandardMacros.DoOnce` false
    (:`Completed`
      (cast `/Game/Characters/Car/BP_MainCharacter` OtherActor)
      (`KismetSystemLibrary.PrintString` "Picked Up Spray Can")
      (`self.Spawn Bull`)
      (`KismetSystemLibrary.Delay` 0.2)
      (`self.K2_DestroyActor`))))

(event `Spawn Bull`
  (`|SpawnActorFromClass` "/Game/Blueprints/Enemy/BP_Bull.BP_Bull_C" (`KismetMathLibrary.MakeTransform` (`SceneComponent.K2_GetComponentLocation` (`self.Start Point`))) "Undefined" "MultiplyWithRoot" null null))

(fn `UserConstructionScript`)