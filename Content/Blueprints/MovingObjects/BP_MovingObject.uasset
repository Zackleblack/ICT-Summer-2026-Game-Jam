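; BP_MovingObject is a moving world object that can optionally kill the player character on contact.
; Its construction script copies the behaviour type, duration and control points into an InterpToMovement component, which drives the motion.
; When a BP_MainCharacter overlaps its Box while Killable is set, it calls DrownDeath on that character unless already dead.
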(event `self.Box.OnComponentBeginOverlap`
  (params (OverlappedComponent :type "PrimitiveComponent Object Reference") (OtherActor :type "Actor Object Reference") (OtherComp :type "PrimitiveComponent Object Reference") (OtherBodyIndex :type Integer) (bFromSweep :type Boolean) (SweepResult :type "HitResult Structure (by ref)"))
  (bind _asbp_main_character (cast `/Game/Characters/Car/BP_MainCharacter` OtherActor))
  (if (`self.bKillable?`)
    (if (not (`/Game/Characters/Car/BP_MainCharacter.bIsDead?` _asbp_main_character))
      (`/Game/Characters/Car/BP_MainCharacter.Drown Death` _asbp_main_character))))

(fn `UserConstructionScript`
  (set `InterpToMovementComponent.BehaviourType` (`self.Behaviour Type`) (`self.InterpToMovement`))
  (set `InterpToMovementComponent.Duration` (`self.Duration`) (`self.InterpToMovement`))
  (set `InterpToMovementComponent.ControlPoints` (`self.Control Points`) (`self.InterpToMovement`)))