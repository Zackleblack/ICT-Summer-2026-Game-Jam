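; BP_Goose is a moving flock of geese that reacts when the player character runs into it.
; The geese loop a run animation from BeginPlay, while a box overlap with BP_MainCharacter calls its AnimalHit once and triggers the flock's hit event.
; That event plays a random-pitch explosion sound, stops InterpToMovement, flattens the geese slightly, halts their animation and destroys the actor after a short delay.
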(event `self.ReceiveBeginPlay`
  (`parent.ReceiveBeginPlay`)
  (`SkeletalMeshComponent.PlayAnimation` (`self.Geese`) "/Game/SM_Models/Geese/GooseRun_Anim.GooseRun_Anim" true)
  (`SkeletalMeshComponent.PlayAnimation` (`self.Geese2`) "/Game/SM_Models/Geese/GooseRun_Anim.GooseRun_Anim" true)
  (`SkeletalMeshComponent.PlayAnimation` (`self.Geese3`) "/Game/SM_Models/Geese/GooseRun_Anim.GooseRun_Anim" true)
  (`SkeletalMeshComponent.PlayAnimation` (`self.Geese4`) "/Game/SM_Models/Geese/GooseRun_Anim.GooseRun_Anim" true)
  (`SkeletalMeshComponent.PlayAnimation` (`self.Geese5`) "/Game/SM_Models/Geese/GooseRun_Anim.GooseRun_Anim" true)
  (`SkeletalMeshComponent.PlayAnimation` (`self.Geese6`) "/Game/SM_Models/Geese/GooseRun_Anim.GooseRun_Anim" true)
  (`SkeletalMeshComponent.PlayAnimation` (`self.Geese7`) "/Game/SM_Models/Geese/GooseRun_Anim.GooseRun_Anim" true)
  (`SkeletalMeshComponent.PlayAnimation` (`self.Geese8`) "/Game/SM_Models/Geese/GooseRun_Anim.GooseRun_Anim" true)
  (`SkeletalMeshComponent.PlayAnimation` (`self.Geese1`) "/Game/SM_Models/Geese/GooseRun_Anim.GooseRun_Anim" true))

(event `self.Box.OnComponentBeginOverlap`
  (params (OverlappedComponent :type "PrimitiveComponent Object Reference") (OtherActor :type "Actor Object Reference") (OtherComp :type "PrimitiveComponent Object Reference") (OtherBodyIndex :type Integer) (bFromSweep :type Boolean) (SweepResult :type "HitResult Structure (by ref)"))
  (bind _asbp_main_character (cast `/Game/Characters/Car/BP_MainCharacter` OtherActor))
  (`|ExecutionSequence`
    (:`then_0`
      (`/Engine/EditorBlueprintResources/StandardMacros.DoOnce` false
        (:`Completed`
          (`/Game/Characters/Car/BP_MainCharacter.Animal Hit` _asbp_main_character))))
    (:`then_1`
      (`self.player hit`))))

(event `player hit`
  (bind _geese (`self.Geese`))
  (`GameplayStatics.PlaySound2D` "/Game/Audio/Explosion.Explosion" 0.5 (`KismetMathLibrary.RandomFloat`) 0.0 null null)
  (`InterpToMovementComponent.StopSimulating` (`self.InterpToMovement`) (stale `self.Box.OnComponentBeginOverlap` SweepResult))
  (`SceneComponent.SetWorldScale3D` _geese (- (`SceneComponent.RelativeScale3D` _geese) (0.0 0.0 0.1)))
  (`SceneComponent.SetWorldScale3D` (`self.Geese2`) (- (`SceneComponent.RelativeScale3D` _geese) (0.0 0.0 0.1)))
  (`SceneComponent.SetWorldScale3D` (`self.Geese3`) (- (`SceneComponent.RelativeScale3D` _geese) (0.0 0.0 0.1)))
  (`SceneComponent.SetWorldScale3D` (`self.Geese4`) (- (`SceneComponent.RelativeScale3D` _geese) (0.0 0.0 0.1)))
  (`SceneComponent.SetWorldScale3D` (`self.Geese5`) (- (`SceneComponent.RelativeScale3D` _geese) (0.0 0.0 0.1)))
  (`SceneComponent.SetWorldScale3D` (`self.Geese6`) (- (`SceneComponent.RelativeScale3D` _geese) (0.0 0.0 0.1)))
  (`SceneComponent.SetWorldScale3D` (`self.Geese7`) (- (`SceneComponent.RelativeScale3D` _geese) (0.0 0.0 0.1)))
  (`SceneComponent.SetWorldScale3D` (`self.Geese8`) (- (`SceneComponent.RelativeScale3D` _geese) (0.0 0.0 0.1)))
  (`SceneComponent.SetWorldScale3D` (`self.Geese1`) (- (`SceneComponent.RelativeScale3D` _geese) (0.0 0.0 0.1)))
  (`SkeletalMeshComponent.Stop` _geese)
  (`SkeletalMeshComponent.Stop` (`self.Geese2`))
  (`SkeletalMeshComponent.Stop` (`self.Geese3`))
  (`SkeletalMeshComponent.Stop` (`self.Geese4`))
  (`SkeletalMeshComponent.Stop` (`self.Geese5`))
  (`SkeletalMeshComponent.Stop` (`self.Geese6`))
  (`SkeletalMeshComponent.Stop` (`self.Geese7`))
  (`SkeletalMeshComponent.Stop` (`self.Geese8`))
  (`SkeletalMeshComponent.Stop` (`self.Geese1`))
  (`KismetSystemLibrary.Delay` 2.0)
  (`self.K2_DestroyActor`))

(fn `UserConstructionScript`
  (`parent.UserConstructionScript`))