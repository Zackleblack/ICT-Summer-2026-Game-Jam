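; Deer obstacle that gallops along configurable InterpToMovement control points until it charges at the player's character.
; When the player enters its Sight volume, it stops, adds audio, resets mesh yaw and shows a warning path faded through a dynamic material.
; After a short delay, a timeline drives it along negative world X, without homing, then destroys it.
; Its Hitbox calls AnimalHit on the player once and plays an explosion sound.
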(event `self.ReceiveBeginPlay`
  (`SkeletalMeshComponent.PlayAnimation` (`self.SkeletalMesh`) "/Game/SM_Models/Deer/MyDeerGallop.MyDeerGallop" true))

(event `self.Hitbox.OnComponentBeginOverlap`
  (params (OverlappedComponent :type "PrimitiveComponent Object Reference") (OtherActor :type "Actor Object Reference") (OtherComp :type "PrimitiveComponent Object Reference") (OtherBodyIndex :type Integer) (bFromSweep :type Boolean) (SweepResult :type "HitResult Structure (by ref)"))
  (bind _asbp_main_character (cast `/Game/Characters/Car/BP_MainCharacter` OtherActor))
  (`/Engine/EditorBlueprintResources/StandardMacros.DoOnce` false
    (:`Completed`
      (`/Game/Characters/Car/BP_MainCharacter.Animal Hit` _asbp_main_character)
      (`self.Player Got Hit`))))

(event `self.Sight.OnComponentBeginOverlap`
  (params (OverlappedComponent :type "PrimitiveComponent Object Reference") (OtherActor :type "Actor Object Reference") (OtherComp :type "PrimitiveComponent Object Reference") (OtherBodyIndex :type Integer) (bFromSweep :type Boolean) (SweepResult :type "HitResult Structure (by ref)"))
  (cast `/Game/Characters/Car/BP_MainCharacter` OtherActor)
  (`self.Look at player`)
  (`SkeletalMeshComponent.Stop` (`self.SkeletalMesh`)))

(event `Look at player`
  (bind _skeletalmesh (`self.SkeletalMesh`))
  (bind (_relativerotation_roll _relativerotation_pitch) (`KismetMathLibrary.BreakRotator` (`SceneComponent.RelativeRotation` _skeletalmesh)))
  (`InterpToMovementComponent.StopSimulating` (`self.InterpToMovement`) (stale `self.Sight.OnComponentBeginOverlap` SweepResult))
  (`AddComponent|NODE_AddAudioComponent-0`)
  (`SceneComponent.K2_SetRelativeRotation` _skeletalmesh (`KismetMathLibrary.MakeRotator` _relativerotation_roll _relativerotation_pitch) false false)
  (`self.Run at player`))

(event `Run at player`
  (bind _returnvalue (`self.K2_GetActorLocation`))
  (`SceneComponent.SetHiddenInGame` (`self.Path`) false false)
  (`|ExecutionSequence`
    (:`then_0`
      (`KismetSystemLibrary.Delay` 1.0)
      (`SkeletalMeshComponent.PlayAnimation` (`self.SkeletalMesh`) "/Game/SM_Models/Deer/MyDeerGallop.MyDeerGallop" true)
      (bind (_direction _newtrack_0) (`Timeline|Timeline`)
        (:`Update`
          (`self.K2_SetActorLocation` (`KismetMathLibrary.VLerp` _returnvalue (- _returnvalue (400.0 0.0 0.0)) _newtrack_0)))
        (:`Finished`
          (`self.K2_DestroyActor`))))
    (:`then_1`
      (bind _returnvalue_2 (`PrimitiveComponent.CreateDynamicMaterialInstance` (`self.Path`) 0 "/Game/Blueprints/Enemy/M_Warning.M_Warning" "None"))
      (bind (_direction_2 _fade_effect) (`Timeline|Timeline_0`)
        (:`Update`
          (`MaterialInstanceDynamic.SetScalarParameterValue` _returnvalue_2 "Fade" _fade_effect))))))

(event `Player Got Hit`
  (`/Engine/EditorBlueprintResources/StandardMacros.DoOnce` false
    (:`Completed`
      (`self.SetActorHiddenInGame` self false)
      (`GameplayStatics.PlaySound2D` "/Game/Audio/Explosion.Explosion" 0.5 (`KismetMathLibrary.RandomFloat`) 0.0 null null))))

(fn `UserConstructionScript`
  (set `InterpToMovementComponent.BehaviourType` (`self.Behaviour Type`) (`self.InterpToMovement`))
  (set `InterpToMovementComponent.Duration` (`self.Duration`) (`self.InterpToMovement`))
  (set `InterpToMovementComponent.ControlPoints` (`self.Control Points`) (`self.InterpToMovement`)))