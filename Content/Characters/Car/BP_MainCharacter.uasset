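; Player character that moves by hopping along world X/Y axes, with a higher leap on a separate input.
; On controller change it adds the IMC_CETA3D mapping context; movement input snaps the mesh to one of four facings, favoring X input, then hops.
; Hop and leap use LaunchCharacter along the mesh's right vector by LeapDistance, and both inputs require being grounded.
; A one-shot Death event sets IsDead and prints a message.
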(event `self.ReceiveControllerChanged`
  (params (OldController :type "Controller Object Reference") (NewController :type "Controller Object Reference"))
  ;[0.1719 0.01729 0.02386] Connected Input System
  (bind _asbp_ceta3d (cast `/Game/Characters/Car/BP_CETA3D` NewController))
  (`EnhancedInputSubsystemInterface.AddMappingContext` (pcsubsystem `EnhancedInputLocalPlayerSubsystem` _asbp_ceta3d) "/Game/Characters/Car/Inputs/IMC_CETA3D.IMC_CETA3D" 0 (struct)))

(event `EnhancedInput|/Game/Characters/Car/Inputs/IA_Movement`
  (params (ActionValue :type "Vector2D Structure") (ElapsedSeconds :type "Float (double-precision)") (TriggeredSeconds :type "Float (double-precision)") (InputAction :type "InputAction Object Reference" :default "/Game/Characters/Car/Inputs/IA_Movement.IA_Movement"))
  ; Movement
  (:`Triggered`
    (if (not (`NavMovementComponent.IsFalling` (`self.CharacterMovement`)))
      (`self.Calculate_Player_Rotation` ActionValue_X ActionValue_Y)
      (if (!= ActionValue_X 0.0)
        (`self.AddMovementInput` (0.0 1.0 0.0) ActionValue_X)
        (`self.Hop`)
        (elif (!= ActionValue_Y 0.0)
          (`self.AddMovementInput` (1.0 0.0 0.0) ActionValue_Y)
          (`self.Hop`))))))

(event `Hop`
  (bind (_returnvalue_x _returnvalue_y) (`KismetMathLibrary.BreakVector` (`SceneComponent.GetRightVector` (`self.Mesh`))))
  ; Movement
  (`self.LaunchCharacter` (`KismetMathLibrary.MakeVector` (* _returnvalue_x (`self.Leap_Distance`)) (* _returnvalue_y (`self.Leap_Distance`)) 200.0) true true))

(event `EnhancedInput|/Game/Characters/Car/Inputs/IA_Leap`
  (params (ActionValue :type Boolean) (ElapsedSeconds :type "Float (double-precision)") (TriggeredSeconds :type "Float (double-precision)") (InputAction :type "InputAction Object Reference" :default "/Game/Characters/Car/Inputs/IA_Leap.IA_Leap"))
  (bind (_returnvalue_x _returnvalue_y) (`KismetMathLibrary.BreakVector` (`SceneComponent.GetRightVector` (`self.Mesh`))))
  ; Leap Mechanic
  (:`Triggered`
    (if (not (`NavMovementComponent.IsFalling` (`self.CharacterMovement`)))
      (`self.LaunchCharacter` (`KismetMathLibrary.MakeVector` (* _returnvalue_x (`self.Leap_Distance`)) (* _returnvalue_y (`self.Leap_Distance`)) 500.0) true true))))

(event `Death`
  (if (not (`self.bIsDead?`))
    (set `self.bIsDead?` true)
    (`KismetSystemLibrary.PrintString` "You Died")))

(fn `Calculate_Player_Rotation`
  (params (`X Axis` :type "Float (double-precision)") (`Y Axis` :type "Float (double-precision)"))
  (if (> `X Axis` 0.0)
    (`SceneComponent.K2_SetRelativeRotation` :`self` (`self.Mesh`))
    (elif (< `X Axis` 0.0)
      (`SceneComponent.K2_SetRelativeRotation` (`self.Mesh`) (struct :`Yaw` 180.0) false false)
      (elif (> `Y Axis` 0.0)
        (`SceneComponent.K2_SetRelativeRotation` (`self.Mesh`) (struct :`Yaw` 270.0) false false)
        (elif true
          (`SceneComponent.K2_SetRelativeRotation` (`self.Mesh`) (struct :`Yaw` 90.0) false false))))))

(fn `UserConstructionScript`)